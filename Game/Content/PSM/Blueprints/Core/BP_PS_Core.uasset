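; BP_PS_Core is a player state Blueprint that stores a player's team ID and team color, with a setter event and a getter.
; On BeginPlay it binds to OnPawnSet, so each pawn change calls OnUpdateTeam, which casts the pawn to BP_Character and calls SRUpdateTeam on it.
; SetTeam only stores the values and does not itself trigger that character update.
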(event `self.ReceiveBeginPlay`
  (add `self.OnPawnSet` (delegate `AssignInitialTeam`)))

(event `AssignInitialTeam` :!signature `self.OnPawnSet`
  (params (Player :type "PlayerState Object Reference") (NewPawn :type "Pawn Object Reference") (OldPawn :type "Pawn Object Reference"))
  (`self.OnUpdateTeam`))

(event `/Game/PSM/Blueprints/Interfaces/BPI_PS_Match.SetTeam`
  (params (TeamId :type String) (TeamColor :type "LinearColor Structure"))
  (set `self.TeamId` TeamId)
  (set `self.CurrentTeam` TeamColor))

(fn `GetTeam`
  (returns (TeamId :type String) (TeamColor :type "LinearColor Structure"))
  (return (`self.TeamId`) (`self.CurrentTeam`)))

(fn `OnUpdateTeam`
  (bind _asbp_character (cast `/Game/PSM/Blueprints/Core/BP_Character` (`self.GetPawn`)))
  (`/Game/PSM/Blueprints/Core/BP_Character.SR_UpdateTeam` _asbp_character))

(fn `UserConstructionScript`)