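; Core game mode that splits joining players into two colored teams and spawns their characters.
; It tracks match controllers on login, controller swap and logout, alternating each new player between Home and Away through the PlayerState.
; After a short delay it replaces any existing pawn with a possessed BP_Character at a random PlayerStart.
; It then calls SRUpdateTeam on tracked players' characters to refresh team data across the match.
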(event `self.K2_PostLogin`
  (params (NewPlayer :type "PlayerController Object Reference"))
  ;[0 0 0] Player Joined Match
  (`KismetArrayLibrary.Array_Add` (`self.MatchPCs`) NewPlayer))

(event `self.HandleStartingNewPlayer`
  (params (NewPlayer :type "PlayerController Object Reference"))
  ;[0 0 0] Spawning & Team Replication
  (`self.Flip Flop Teams` NewPlayer)
  (`KismetSystemLibrary.Delay` 0.5)
  (`self.SpawnPlayer` NewPlayer)
  (`self.AssignTeams`))

(event `self.K2_OnSwapPlayerControllers`
  (params (OldPC :type "PlayerController Object Reference") (NewPC :type "PlayerController Object Reference"))
  ;[0 0 0] Player Joined Match
  (`KismetArrayLibrary.Array_Add` (`self.MatchPCs`) NewPC))

(event `self.K2_OnLogout`
  (params (ExitingController :type "Controller Object Reference"))
  ;[0 0 0] Player Exit Match
  (bind _asplayer_controller (cast `PlayerController` ExitingController))
  (`KismetArrayLibrary.Array_RemoveItem` (`self.MatchPCs`) _asplayer_controller))

(fn `AssignTeams`
  (for _array_element (`self.MatchPCs`)
    (bind _asbp_character (cast `/Game/PSM/Blueprints/Core/BP_Character` (`Controller.K2_GetPawn` _array_element)))
    (`/Game/PSM/Blueprints/Core/BP_Character.SR_UpdateTeam` _asbp_character)))

(fn `Flip Flop Teams`
  (params (PlayerController :type "PlayerController Object Reference (by ref)"))
  (locals (PlayerState :type "PlayerState Object Reference"))
  (bind _playerstate (`local.PlayerState`))
  (set `local.PlayerState` (`Controller.PlayerState` PlayerController))
  (if (== (`self.LastTeamAssign`) (struct :`R` 0.009419 :`G` 0.223296 :`B` 1.0 :`A` 1.0))
    (bind _output_get (set `self.LastTeamAssign` (struct :`R` 1.0 :`G` 0.039546 :`B` 0.039546 :`A` 1.0)))
    (message `/Game/PSM/Blueprints/Interfaces/BPI_PS_Match.SetTeam` _playerstate "Home Team" _output_get)
    (else
      (bind _output_get_2 (set `self.LastTeamAssign` (struct :`R` 0.009419 :`G` 0.223296 :`B` 1.0 :`A` 1.0)))
      (message `/Game/PSM/Blueprints/Interfaces/BPI_PS_Match.SetTeam` _playerstate "Away Team" _output_get_2))))

(fn `GetRandomSpawnPoint`
  (returns (SpawnTransform :type "Transform Structure (by ref)"))
  (bind _outactors (`GameplayStatics.GetAllActorsOfClass` "/Script/Engine.PlayerStart"))
  (return (`self.GetTransform` (`|GetArrayItem` _outactors (`KismetMathLibrary.RandomIntegerInRange` 0 (- (`KismetArrayLibrary.Array_Length` _outactors) 1))))))

(fn `SpawnPlayer`
  (params (PlayerController :type "PlayerController Object Reference"))
  (locals (PlayerState :type "PlayerState Object Reference"))
  (bind _returnvalue (`Controller.K2_GetPawn` (`local.PlayerController`)))
  (set `local.PlayerState` (`Controller.PlayerState` PlayerController))
  (`/Engine/EditorBlueprintResources/StandardMacros.IsValid` _returnvalue
    (:`Is Valid`
      (`self.K2_DestroyActor` _returnvalue))
    (:`Is Not Valid`
      _))
  (bind _returnvalue_2 (`|SpawnActorFromClass` "/Game/PSM/Blueprints/Core/BP_Character.BP_Character_C" (`self.GetRandomSpawnPoint`) "Undefined" "OverrideRootScale" null null))
  (`Controller.Possess` (`local.PlayerController`) _returnvalue_2))

(fn `UserConstructionScript`)