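; Core HUD class that creates, shows and switches the player's UI widgets.
; On BeginPlay it sets game-only input, instantiates the CreateWidgets map's classes into WidgetList and adds them to the viewport.
; Creation collapses every widget when the map's first value is true, ignoring each entry's own flag.
; ToggleWidget shows or hides the target, collapses the others, and switches input mode and mouse cursor accordingly.
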(event `self.ReceiveBeginPlay`
  (`WidgetBlueprintLibrary.SetInputMode_GameOnly` (`self.GetOwningPlayerController`))
  (`self.Add UIWidgets` (`self.CreateWidgets`))
  (for _array_element (`self.WidgetList`)
    (`UserWidget.AddToViewport` _array_element 0)))

(fn `Add UIWidgets`
  (params (WidgetsClass :type "Map of UserWidget Class Reference to Boolean"))
  (bind _keys (`BlueprintMapLibrary.Map_Keys` WidgetsClass))
  (for _array_element _keys
    (bind _returnvalue (`|CreateWidget` _array_element (`self.GetOwningPlayerController`)))
    (`KismetArrayLibrary.Array_Add` (`self.WidgetList`) _returnvalue)
    (bind _values (`BlueprintMapLibrary.Map_Values` (`local.WidgetsClass`)))
    (if (`|GetArrayItem` _values)
      (`Widget.SetVisibility` _returnvalue "Collapsed"))))

(fn `FocusGame`
  (bind _returnvalue (`self.GetOwningPlayerController`))
  (`Widget.SetVisibility` (`self.ActiveWidget`) "Collapsed")
  (`WidgetBlueprintLibrary.SetInputMode_GameOnly` _returnvalue)
  (set `PlayerController.bShowMouseCursor` false _returnvalue))

(fn `FocusWidget`
  (bind _returnvalue (`self.GetOwningPlayerController`))
  (bind _activewidget (`self.ActiveWidget`))
  (`Widget.SetVisibility` _activewidget "SelfHitTestInvisible")
  (`WidgetBlueprintLibrary.SetInputMode_GameAndUIEx` _returnvalue _activewidget)
  (set `PlayerController.bShowMouseCursor` true _returnvalue))

(fn `ToggleWidget`
  (params (TargetWidget :type "UserWidget Object Reference"))
  (`/Engine/EditorBlueprintResources/StandardMacros.IsValid` TargetWidget
    (:`Is Valid`
      (set `self.ActiveWidget` TargetWidget)
      (for _array_element (`self.WidgetList`)
        (`/Engine/EditorBlueprintResources/StandardMacros.IsValid` _array_element
          (:`Is Valid`
            (if (== (`self.ActiveWidget`) _array_element)
              (if (`Widget.IsVisible` (`self.ActiveWidget`))
                (`self.FocusGame`)
                (else
                  (`self.FocusWidget`)))
              (elif (`Widget.IsVisible` _array_element)
                (`Widget.SetVisibility` _array_element "Collapsed")))))))))

(fn `UserConstructionScript`)