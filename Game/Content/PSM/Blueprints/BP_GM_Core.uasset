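; Core game mode Blueprint that tracks the player controllers in a match and provides player spawning.
; Login and controller-swap events add controllers to MatchPCs, and logout removes them.
; SpawnPlayer destroys the controller's current pawn, then spawns and possesses a new third-person character at a randomly chosen PlayerStart.
; Nothing in this graph calls SpawnPlayer, and a swap does not remove the old controller from the list.
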(event `self.K2_PostLogin`
  (params (NewPlayer :type "PlayerController Object Reference"))
  ;[0 0 0] Player Joined Match
  (`KismetArrayLibrary.Array_Add` (`self.MatchPCs`) NewPlayer))

(event `self.K2_OnSwapPlayerControllers`
  (params (OldPC :type "PlayerController Object Reference") (NewPC :type "PlayerController Object Reference"))
  ;[0 0 0] Player Joined Match
  (`KismetArrayLibrary.Array_Add` (`self.MatchPCs`) NewPC))

(event `self.K2_OnLogout`
  (params (ExitingController :type "Controller Object Reference"))
  ;[0 0 0] Player Exit Match
  (bind _asplayer_controller (cast `PlayerController` ExitingController))
  (`KismetArrayLibrary.Array_RemoveItem` (`self.MatchPCs`) _asplayer_controller))

(fn `GetRandomSpawnPoint`
  (returns (SpawnTransform :type "Transform Structure (by ref)"))
  (bind _outactors (`GameplayStatics.GetAllActorsOfClass` "/Script/Engine.PlayerStart"))
  (return (`self.GetTransform` (`|GetArrayItem` _outactors (`KismetMathLibrary.RandomIntegerInRange` 0 (- (`KismetArrayLibrary.Array_Length` _outactors) 1))))))

(fn `SpawnPlayer`
  (params (PlayerController :type "PlayerController Object Reference"))
  (bind _returnvalue (`Controller.K2_GetPawn` PlayerController))
  (`/Engine/EditorBlueprintResources/StandardMacros.IsValid` _returnvalue
    (:`Is Valid`
      (`self.K2_DestroyActor` _returnvalue))
    (:`Is Not Valid`
      _))
  (bind _returnvalue_2 (`|SpawnActorFromClass` "/Game/Engine/ThirdPerson/Blueprints/BP_ThirdPersonCharacter.BP_ThirdPersonCharacter_C" (`self.GetRandomSpawnPoint`) "Undefined" "OverrideRootScale" null null))
  (`Controller.Possess` (`local.PlayerController`) _returnvalue_2))

(fn `UserConstructionScript`)